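; BP_LockedDoor is a door that opens on interaction, requiring a key item when locked.
; For a locked door, Interact casts the caller to ItemSystemCharacter, checks its InventoryComponent for RequiredKeyID, then consumes the key and unlocks, or prints a Korean key-needed message.
; Opening plays a timeline that lerps HingePoint's relative yaw to OpenAngle, and IsOpen blocks further interaction, so the door never closes.
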(event `InteractInterface.Interact`
  (params (Caller :type "Actor Object Reference"))
  (if (`self.bIsOpen`)
    _
    (elif (`self.bIsLocked`)
      (bind _asitem_system_character (cast `ItemSystemCharacter` Caller))
      (bind _inventorycomponent (`ItemSystemCharacter.InventoryComponent` _asitem_system_character))
      (if (`InventoryComponent.HasItem` _inventorycomponent (`self.RequiredKeyID`))
        (`InventoryComponent.RemoveItem` _inventorycomponent (`self.RequiredKeyID`))
        (set `self.bIsLocked` false)
        (set `self.bIsOpen` true :!label _label)
        (bind (_direction _dooralpha) (`Timeline|DoorTimeLine`)
          (:`Update`
            (`SceneComponent.K2_SetRelativeRotation` (`self.HingePoint`) (`KismetMathLibrary.RLerp` (struct) (`KismetMathLibrary.MakeRotator` 0.0 0.0 (`self.OpenAngle`)) _dooralpha) false false)))
        (else
          (`KismetSystemLibrary.PrintString` "열쇠가 필요합니다")))
      (else
        (goto _label)))))

(fn `UserConstructionScript`)