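; BP_DamageZone is an area hazard that deals continuous damage to the player standing inside it.
; DamageArea overlap events toggle an in-zone flag whenever an ItemSystemCharacter enters or leaves.
; While the flag is set, Tick applies DamagePerSecond scaled by delta time to the StatusComponent of player character 0, rather than to the actor that overlapped.
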(event `self.DamageArea.OnComponentBeginOverlap`
  (params (OverlappedComponent :type "PrimitiveComponent Object Reference") (OtherActor :type "Actor Object Reference") (OtherComp :type "PrimitiveComponent Object Reference") (OtherBodyIndex :type Integer) (bFromSweep :type Boolean) (SweepResult :type "HitResult Structure (by ref)"))
  (cast `ItemSystemCharacter` OtherActor)
  (set `self.bIsPlayerInZone` true))

(event `self.DamageArea.OnComponentEndOverlap`
  (params (OverlappedComponent :type "PrimitiveComponent Object Reference") (OtherActor :type "Actor Object Reference") (OtherComp :type "PrimitiveComponent Object Reference") (OtherBodyIndex :type Integer))
  (cast `ItemSystemCharacter` OtherActor)
  (set `self.bIsPlayerInZone` false))

(event `self.ReceiveTick`
  (params (DeltaSeconds :type "Float (single-precision)"))
  (if (`self.bIsPlayerInZone`)
    (bind _asitem_system_character (cast `ItemSystemCharacter` (`GameplayStatics.GetPlayerCharacter` 0)))
    (`StatusComponent.ApplyDamage` (`ItemSystemCharacter.StatusComponent` _asitem_system_character) (* (`self.DamagePerSecond`) DeltaSeconds))))

(fn `UserConstructionScript`)